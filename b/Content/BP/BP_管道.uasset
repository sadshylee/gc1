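; Pipe actor (BP_管道) that builds a spline-mesh pipe with rounded corners along an editable spline.
; The construction script makes Spline1 linear, then 生成样条线 builds a second spline, splitting inner points at ±转角距离 and setting scaled tangents to round bends.
; 生成管道 adds a mesh segment between each point pair, applying material and thickness (粗细).
; Tick also plays a timeline whose updates rerun 生成管道, adding segments without clearing earlier ones.
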(event `self.ReceiveTick`
  (params (DeltaSeconds :type "Float (single-precision)"))
  (`Timeline|时间轴`
    (:`Update`
      (`self.生成管道`))))

(fn `UserConstructionScript`
  (bind _spline1 (`self.Spline1`))
  (`|ExecutionSequence`
    (:`then_0`
      (for _index (range (+ (- (`SplineComponent.GetNumberOfSplinePoints` _spline1) 2) 1))
        (`SplineComponent.SetSplinePointType` _spline1 _index "Linear" true)))
    (:`then_1`
      (`self.生成样条线`))
    (:`then_2`
      (`self.生成管道`))))

(fn `生成样条线`
  (bind `_新样条点` (`self.新样条点`))
  (bind _spline1 (`self.Spline1`))
  (bind `_转角距离` (`self.转角距离`))
  (bind _spline1_2 (`self.Spline1`))
  (bind _spline1_3 (`self.Spline1`))
  (bind _spline1_4 (`self.Spline1`))
  (bind _returnvalue (`SplineComponent.GetDistanceAlongSplineAtSplinePoint` _spline1 (`self.Index`)))
  (bind _returnvalue_2 (- (`SplineComponent.GetNumberOfSplinePoints` (`self.Spline1`)) 1))
  (bind _returnvalue_3 (- _returnvalue `_转角距离`))
  (bind _returnvalue_4 (+ _returnvalue `_转角距离`))
  (bind _returnvalue_5 (`AddComponent|NODE_AddSplineComponent-0`))
  (bind _output_get (set `self.新样条点` _returnvalue_5))
  (`SplineComponent.ClearSplinePoints` _output_get true)
  (for _index (range (`SplineComponent.GetNumberOfSplinePoints` (`self.Spline1`)))
    (set `self.Index` _index)
    (if (== _index 0)
      (`SplineComponent.AddSplinePoint` (`self.新样条点`) (`SplineComponent.GetLocationAtSplinePoint` _spline1_3 0 "Local") "Local" true)
      (`KismetArrayLibrary.Array_Add` (`self.In Tangent`) (`SplineComponent.GetTangentAtSplinePoint` _spline1_3 0 "Local"))
      (elif (== _index (- (`SplineComponent.GetNumberOfSplinePoints` (`self.Spline1`)) 1))
        (`SplineComponent.AddSplinePoint` (`self.新样条点`) (`SplineComponent.GetLocationAtSplinePoint` _spline1_4 _returnvalue_2 "Local") "Local" true)
        (`KismetArrayLibrary.Array_Add` (`self.In Tangent`) (`SplineComponent.GetTangentAtSplinePoint` _spline1_4 _returnvalue_2 "Local"))
        (else
          (`SplineComponent.AddSplinePoint` `_新样条点` (`SplineComponent.GetLocationAtDistanceAlongSpline` _spline1 _returnvalue_3 "Local") "Local" true)
          (`KismetArrayLibrary.Array_Add` (`self.In Tangent`) (`SplineComponent.GetTangentAtDistanceAlongSpline` _spline1_2 _returnvalue_3 "Local"))
          (`SplineComponent.AddSplinePoint` `_新样条点` (`SplineComponent.GetLocationAtDistanceAlongSpline` _spline1 _returnvalue_4 "Local") "Local" true)
          (`KismetArrayLibrary.Array_Add` (`self.In Tangent`) (`SplineComponent.GetTangentAtDistanceAlongSpline` _spline1_2 _returnvalue_4 "Local"))))))
  (for _index_2 (range (+ (`SplineComponent.GetNumberOfSplinePoints` (`self.新样条点`)) 1))
    (`SplineComponent.SetTangentAtSplinePoint` (`self.新样条点`) _index_2 (* (`KismetMathLibrary.Normal` (`|GetArrayItem` (`self.In Tangent`) _index_2)) (* (`self.转角距离`) 2.0)) "Local" true)))

(fn `生成管道`
  (bind `_粗细` (`self.粗细`))
  (bind `_新样条点` (`self.新样条点`))
  (for _index (range (+ (- (`SplineComponent.GetNumberOfSplinePoints` (`self.新样条点`)) 2) 1))
    (bind _returnvalue (`AddComponent|NODE_AddSplineMeshComponent-1`))
    (`StaticMeshComponent.SetStaticMesh` _returnvalue (`self.Mesh`))
    (`PrimitiveComponent.SetMaterial` _returnvalue 0 (`self.Material`))
    (bind (_location _tangent) (`SplineComponent.GetLocationAndTangentAtSplinePoint` `_新样条点` _index "Local"))
    (bind (_location_2 _tangent_2) (`SplineComponent.GetLocationAndTangentAtSplinePoint` `_新样条点` (+ _index 1) "Local"))
    (`SplineMeshComponent.SetStartAndEnd` _returnvalue _location _tangent _location_2 _tangent_2 true)
    (`SplineMeshComponent.SetStartScale` _returnvalue (`KismetMathLibrary.MakeVector2D` `_粗细` `_粗细`) true)
    (`SplineMeshComponent.SetEndScale` _returnvalue (`KismetMathLibrary.MakeVector2D` `_粗细` `_粗细`) true)))