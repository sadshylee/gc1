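; BP_实验报告 (experiment report) is an actor that highlights itself and shows a UI widget when its Box trigger is overlapped.
; Begin overlap applies the M_高亮 overlay material to the 显示 component, creates a WB widget, adds it to the viewport and shows the mouse cursor.
; End overlap clears the overlay and removes the stored widget, but leaves the cursor visible.
; Neither event filters the overlapping actor.
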(event `self.Box.OnComponentBeginOverlap`
  (params (OverlappedComponent :type "PrimitiveComponent Object Reference") (OtherActor :type "Actor Object Reference") (OtherComp :type "PrimitiveComponent Object Reference") (OtherBodyIndex :type Integer) (bFromSweep :type Boolean) (SweepResult :type "HitResult Structure (by ref)"))
  (`MeshComponent.SetOverlayMaterial` (`self.显示`) "/Game/mod/BP_mod/M_高亮.M_高亮")
  (bind _returnvalue (`|CreateWidget` "/Game/动画/控件/WB.WB_C"))
  (bind _output_get (set `self.NewVar` _returnvalue))
  (`UserWidget.AddToViewport` _output_get 0)
  (set `PlayerController.bShowMouseCursor` true (`GameplayStatics.GetPlayerController` 0)))

(event `self.Box.OnComponentEndOverlap`
  (params (OverlappedComponent :type "PrimitiveComponent Object Reference") (OtherActor :type "Actor Object Reference") (OtherComp :type "PrimitiveComponent Object Reference") (OtherBodyIndex :type Integer))
  (`MeshComponent.SetOverlayMaterial` (`self.显示`) null)
  (`Widget.RemoveFromParent` (`self.NewVar`)))

(fn `UserConstructionScript`)