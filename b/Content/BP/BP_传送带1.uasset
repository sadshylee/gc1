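; BP_传送带1 is a conveyor belt actor that carries BP_铁团 actors along its direction.
; Each Tick it queries its Box for overlapping BP_铁团 and offsets each one along the Arrow's forward vector by Speed scaled by DeltaSeconds.
; Movement sets world position directly without sweep, so collisions along the path are not checked.
; Debug prints of the overlap count and loop progress run every frame.
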(event `self.ReceiveTick`
  (params (DeltaSeconds :type "Float (single-precision)"))
  (bind _overlappingactors (`PrimitiveComponent.GetOverlappingActors` (`self.Box`) "/Game/BP/BP_铁团.BP_铁团_C"))
  (`KismetSystemLibrary.PrintString` (`KismetStringLibrary.Conv_IntToString` (`KismetArrayLibrary.Array_Length` _overlappingactors)))
  (for _array_element _overlappingactors
    (bind `_asbp_铁团` (cast `/Game/BP/BP_铁团` _array_element))
    (`KismetSystemLibrary.PrintString` "shibai")
    (`KismetSystemLibrary.PrintString` "Hello")
    (`self.K2_AddActorWorldOffset` `_asbp_铁团` (* (* DeltaSeconds (`self.speed`)) (`SceneComponent.GetForwardVector` (`self.Arrow`))) false false)))

(fn `UserConstructionScript`)