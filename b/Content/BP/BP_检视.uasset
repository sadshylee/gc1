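; BP_检视 is an inspectable item that opens an inspection view when the player interacts with it.
; The construction script applies the configured mesh and scale to Cube, and highlight events toggle an overlay material on it.
; If 是否检视 is set, Oninteract spawns BP_检视界面 at a far-off world location, then passes it the initial rotation, orientation, mesh, name, description, image and interacting character.
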(event `/Game/BP/函数库/物品显示接口.打开高亮`
  (`MeshComponent.SetOverlayMaterial` (`self.Cube`) "/Game/mod/BP_mod/M_高亮.M_高亮"))

(event `/Game/BP/函数库/物品显示接口.关闭高亮`
  (`MeshComponent.SetOverlayMaterial` (`self.Cube`) null))

(event `self.ReceiveBeginPlay`
  (set `self.Player Ref` (`/Game/BP/函数库/BPFL_检视.FIP_GetPlayRef`)))

(event `/Game/BP/函数库/BPL_检视.Oninteract`
  (params (`角色` :type "/Game/ThirdPerson/Blueprints/BP_ThirdPersonCharacter Object Reference"))
  (if (`self.是否检视`)
    (bind _returnvalue (`|SpawnActorFromClass` "/Game/BP/BP_检视界面.BP_检视界面_C" (`KismetMathLibrary.MakeTransform` (100000000000.0 0.0 0.0)) "Undefined" "MultiplyWithRoot" null null))
    (set `/Game/BP/BP_检视界面.初始物品旋转` (`self.旋转`) _returnvalue)
    (set `/Game/BP/BP_检视界面.初始物品方向` (`self.物品方向`) _returnvalue)
    (message `/Game/BP/函数库/BPL_检视.intercat` _returnvalue `角色` (`StaticMeshComponent.StaticMesh` (`self.Cube`)) (`self.物品名字`) (`self.物品描述`) (`self.物品图像`))))

(fn `UserConstructionScript`
  (bind _cube (`self.Cube`))
  (`StaticMeshComponent.SetStaticMesh` _cube (`self.物品网格体`))
  (`SceneComponent.K2_SetWorldTransform` _cube (`KismetMathLibrary.MakeTransform` (`SceneComponent.K2_GetComponentLocation` _cube) (`SceneComponent.K2_GetComponentRotation` _cube) (`self.物品大小`)) false false))