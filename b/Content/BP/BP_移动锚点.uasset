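; BP_移动锚点 is a two-way movement anchor that glides the third-person character between its two pads.
; Overlapping Capsule or Capsule1 runs that side's timeline, lerping the character's location to 地基1 or 地基 respectively, with a height offset and no sweep.
; The 正在传送 flag blocks retriggering until the timeline finishes, but is set before the cast, so another overlapping actor leaves it locked.
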(event `self.Capsule.OnComponentBeginOverlap`
  (params (OverlappedComponent :type "PrimitiveComponent Object Reference") (OtherActor :type "Actor Object Reference") (OtherComp :type "PrimitiveComponent Object Reference") (OtherBodyIndex :type Integer) (bFromSweep :type Boolean) (SweepResult :type "HitResult Structure (by ref)"))
  (if (not (`self.正在传送`))
    (set `self.正在传送` true)
    (bind _asbp_third_person_character (cast `/Game/ThirdPerson/Blueprints/BP_ThirdPersonCharacter` OtherActor))
    (set `self.As BP Third Person Character` _asbp_third_person_character)
    (set `self.初始位置` (+ (`self.K2_GetActorLocation` (`self.As BP Third Person Character`)) (0.0 0.0 30.0)))
    (set `self.目标位置` (+ (`SceneComponent.K2_GetComponentLocation` (`self.地基1`)) (0.0 0.0 30.0)))
    (bind (_direction `_新建轨道_0`) (`Timeline|时间轴`)
      (:`Update`
        (`self.K2_SetActorLocation` (`self.As BP Third Person Character`) (`KismetMathLibrary.VLerp` (`self.初始位置`) (`self.目标位置`) `_新建轨道_0`) false false))
      (:`Finished`
        (set `self.正在传送` false)))))

(event `self.Capsule1.OnComponentBeginOverlap`
  (params (OverlappedComponent :type "PrimitiveComponent Object Reference") (OtherActor :type "Actor Object Reference") (OtherComp :type "PrimitiveComponent Object Reference") (OtherBodyIndex :type Integer) (bFromSweep :type Boolean) (SweepResult :type "HitResult Structure (by ref)"))
  (if (not (`self.正在传送`))
    (set `self.正在传送` true)
    (bind _asbp_third_person_character (cast `/Game/ThirdPerson/Blueprints/BP_ThirdPersonCharacter` OtherActor))
    (set `self.As BP Third Person Character` _asbp_third_person_character)
    (set `self.初始位置` (+ (`self.K2_GetActorLocation` (`self.As BP Third Person Character`)) (0.0 0.0 30.0)))
    (set `self.目标位置` (+ (`SceneComponent.K2_GetComponentLocation` (`self.地基`)) (0.0 0.0 30.0)))
    (bind (_direction `_新建轨道_0`) (`Timeline|时间轴_0`)
      (:`Update`
        (`self.K2_SetActorLocation` (`self.As BP Third Person Character`) (`KismetMathLibrary.VLerp` (`self.初始位置`) (`self.目标位置`) `_新建轨道_0`) false false))
      (:`Finished`
        (set `self.正在传送` false)))))

(fn `UserConstructionScript`)